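; Infinite-terrain tile that fills itself with props and AI characters on BeginPlay, using inherited-style placement calls with per-type spawn arguments.
; Player overlap with the lock trigger opens the barrier (green) and reports the tile conquered to the game mode once; leaving it locks the barrier (red).
; Leaving the destroy trigger asks the game mode to spawn another tile and destroys this one.
; GetAttachLocation exposes the Arrow transform.
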(event `self.ReceiveBeginPlay`
  (`self.Unlock`)
  (`self.PlaceActors` "/Game/Dynamic/Terrain/Props/BP_Container.BP_Container_C" (`self.FSPawnArgument_Container`))
  (`self.PlaceActors` "/Game/Dynamic/Terrain/Props/BP_Box.BP_Box_C" (`self.FSPawnArgument_Box`))
  (`self.PlaceActors` "/Game/Dynamic/Terrain/Props/BP_Canister.BP_Canister_C" (`self.FSPawnArgument_Canister`))
  (`self.PlaceActors` "/Game/Dynamic/Terrain/Props/BP_Rock01.BP_Rock01_C" (`self.FSPawnArgument_Rocks`))
  (`self.PlaceActors` "/Game/Dynamic/Terrain/Props/BP_Rock05.BP_Rock05_C" (`self.FSPawnArgument_Rocks2`))
  (`self.PlaceActors` "/Game/Dynamic/Terrain/Props/BP_Rock17.BP_Rock17_C" (`self.FSPawnArgument_Rocks2`))
  (`self.PlaceActors` "/Game/Dynamic/Terrain/Props/BP_Sack2.BP_Sack2_C" (`self.FSPawnArgument_Sack`))
  (`self.PlaceAIPawns` "/Game/Dynamic/Character/Behaviour/BP_Character.BP_Character_C" (`self.FSPawnArguments_AI`)))

(event `self.Lock_CB.OnComponentBeginOverlap`
  (params (OverlappedComponent :type "PrimitiveComponent Object Reference") (OtherActor :type "Actor Object Reference") (OtherComp :type "PrimitiveComponent Object Reference") (OtherBodyIndex :type Integer) (bFromSweep :type Boolean) (SweepResult :type "HitResult Structure (by ref)"))
  (`self.IsPlayerActor` OtherActor)
  (`|ExecutionSequence`
    (:`then_0`
      (`self.Unlock`))
    (:`then_1`
      (`self.TileConquered`))))

(event `self.Lock_CB.OnComponentEndOverlap`
  (params (OverlappedComponent :type "PrimitiveComponent Object Reference") (OtherActor :type "Actor Object Reference") (OtherComp :type "PrimitiveComponent Object Reference") (OtherBodyIndex :type Integer))
  (`self.IsPlayerActor` OtherActor)
  (`self.Lock`))

(event `self.DestroyTile_CB.OnComponentEndOverlap`
  (params (OverlappedComponent :type "PrimitiveComponent Object Reference") (OtherActor :type "Actor Object Reference") (OtherComp :type "PrimitiveComponent Object Reference") (OtherBodyIndex :type Integer))
  (`self.IsPlayerActor` OtherActor)
  (bind _asbp_infinite_terrain_game_mode (cast `/Game/Dynamic/BP_InfiniteTerrainGameMode` (`GameplayStatics.GetGameMode`)))
  (`/Game/Dynamic/BP_InfiniteTerrainGameMode.SpawnTile` _asbp_infinite_terrain_game_mode)
  (`self.K2_DestroyActor` self))

(fn `GetAttachLocation`
  (returns (AttachTransform :type "Transform Structure"))
  (return (`SceneComponent.K2_GetComponentToWorld` (`self.Arrow`))))

(fn `Lock`
  (`PrimitiveComponent.SetCollisionEnabled` (`self.Barrier`) "QueryAndPhysics")
  (`PrimitiveComponent.SetMaterial` (`self.Barrier`) 0 "/Game/Dynamic/Terrain/MI_Barrier_Red.MI_Barrier_Red"))

(fn `TileConquered`
  (if (not (`self.bIsConquered`))
    (bind _asbp_infinite_terrain_game_mode (cast `/Game/Dynamic/BP_InfiniteTerrainGameMode` (`GameplayStatics.GetGameMode`)))
    (`/Game/Dynamic/BP_InfiniteTerrainGameMode.TileConquered` _asbp_infinite_terrain_game_mode)
    (set `self.bIsConquered` true)))

(fn `Unlock`
  (`PrimitiveComponent.SetCollisionEnabled` (`self.Barrier`) "NoCollision")
  (`PrimitiveComponent.SetMaterial` (`self.Barrier`) 0 "/Game/Dynamic/Terrain/MI_Barrier_Green.MI_Barrier_Green"))

(fn `UserConstructionScript`)