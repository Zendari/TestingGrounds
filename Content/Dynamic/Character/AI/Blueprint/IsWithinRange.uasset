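; IsWithinRange is a Behavior Tree decorator that tests whether an AI pawn is close enough to its target.
; It reads the Target actor from the Blackboard and compares its straight-line 3D distance from the controlled pawn against the Range variable.
; The condition passes at or within that range and fails when the target is invalid.
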(fn `PerformConditionCheckAI`
  (params (OwnerController :type "AIController Object Reference") (ControlledPawn :type "Pawn Object Reference"))
  (returns (ReturnValue :type Boolean))
  (if (`KismetSystemLibrary.IsValid` (`BTFunctionLibrary.GetBlackboardValueAsActor` (`self.Target`)))
    (return (<= (`KismetMathLibrary.VSize` (- (`Actor.K2_GetActorLocation` ControlledPawn) (`Actor.K2_GetActorLocation` (`BTFunctionLibrary.GetBlackboardValueAsActor` (`self.Target`))))) (`self.Range`)))
    (else
      (return false))))