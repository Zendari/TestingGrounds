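; BP_HealBox is a health pickup prop that heals the player character on contact.
; When its static mesh begins overlapping an actor, the IsPlayerActor macro checks that the actor is player 0's character.
; It then calls HealCharacter on BP_Character and destroys itself if that call returns true or the character's HasHealed flag is set.
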(event `self.StaticMesh.OnComponentBeginOverlap`
  (params (OverlappedComponent :type "PrimitiveComponent Object Reference") (OtherActor :type "Actor Object Reference") (OtherComp :type "PrimitiveComponent Object Reference") (OtherBodyIndex :type Integer) (bFromSweep :type Boolean) (SweepResult :type "HitResult Structure (by ref)"))
  ;[1 1 1] OnHit & HealCharacter
  (`self.IsPlayerActor` OtherActor
    (:`True`
      (bind _asbp_character (cast `/Game/Dynamic/Character/Behaviour/BP_Character` OtherActor))
      (bind _hashealed (`/Game/Dynamic/Character/Behaviour/BP_Character.Heal Character` _asbp_character))
      (if (or _hashealed (`/Game/Dynamic/Character/Behaviour/BP_Character.HasHealed` _asbp_character))
        (`self.K2_DestroyActor`)))))

(fn `UserConstructionScript`)