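; AI controller for guard NPCs that tracks sensed targets through AI Perception.
; On BeginPlay it sets up the GuardBehaviour_Data blackboard and runs the GuardBehavior tree.
; Perception updates write any sensed actor lacking the "Enemy" tag to the blackboard's Enemy key, so tagged actors are ignored.
; Failed sensing of an untagged actor clears that key.
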(event `self.ReceiveBeginPlay`
  (bind _blackboardcomponent (`self.UseBlackboard` "/Game/Dynamic/Character/AI/Blueprint/GuardBehaviour_Data.GuardBehaviour_Data"))
  (`self.RunBehaviorTree` "/Game/Dynamic/Character/AI/Blueprint/GuardBehavior.GuardBehavior")
  (set `self.BlackBoardComp` _blackboardcomponent))

(event `self.AIPerception.OnTargetPerceptionUpdated`
  (params (Actor :type "Actor Object Reference") (Stimulus :type "AIStimulus Structure"))
  (`self.UpdateBalckboardEnemyKey` Stimulus Actor Actor))

(fn `UpdateBalckboardEnemyKey`
  (params (AIStimulus :type "AIStimulus Structure (by ref)") (InputPin :type "Actor Object Reference") (self2 :type "Actor Object Reference"))
  (if (`self.ActorHasTag` self2 "Enemy")
    _
    (elif (`.bSuccessfullySensed` (break `AIStimulus` AIStimulus))
      (`BlackboardComponent.SetValueAsObject` (`self.BlackBoardComp`) "Enemy" InputPin)
      (else
        (`BlackboardComponent.ClearValue` (`self.BlackBoardComp`) "Enemy")))))

(fn `UserConstructionScript`)