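; AI controller for guard NPCs that runs the GuardBehavior tree on the GuardBehaviour_Data blackboard.
; Perception updates store sensed actors lacking the "Enemy" tag in the blackboard's Enemy key, and clear it when sensing fails.
; Each tick, it sets the controlled Ue4ASP_Character's aiming and shooting flags according to whether the controller has a valid focus actor.
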(event `self.ReceiveBeginPlay`
  (bind _blackboardcomponent (`self.UseBlackboard` "/Game/Dynamic/NPC/AI/Blueprint/GuardBehaviour_Data.GuardBehaviour_Data"))
  (`self.RunBehaviorTree` "/Game/Dynamic/NPC/AI/Blueprint/GuardBehavior.GuardBehavior")
  (set `self.BlackBoardComp` _blackboardcomponent))

(event `self.AIPerception.OnTargetPerceptionUpdated`
  (params (Actor :type "Actor Object Reference") (Stimulus :type "AIStimulus Structure"))
  (if (`self.ActorHasTag` Actor "Enemy")
    _
    (elif (`.bSuccessfullySensed` (break `AIStimulus` Stimulus))
      (`BlackboardComponent.SetValueAsObject` (`self.BlackBoardComp`) "Enemy" Actor)
      (else
        (`BlackboardComponent.ClearValue` (`self.BlackBoardComp`) "Enemy")))))

(event `self.ReceiveTick`
  (params (DeltaSeconds :type "Float (single-precision)"))
  (bind _returnvalue (`KismetSystemLibrary.IsValid` (`self.GetFocusActor`)))
  (bind _asue_4asp_character (cast `/Game/Dynamic/NPC/Behavioiur/Ue4ASP_Character` (`self.K2_GetPawn`)))
  (set `/Game/Dynamic/NPC/Behavioiur/Ue4ASP_Character.bIsAiming` _returnvalue _asue_4asp_character)
  (set `/Game/Dynamic/NPC/Behavioiur/Ue4ASP_Character.bIsShooting` _returnvalue _asue_4asp_character))

(fn `UserConstructionScript`)